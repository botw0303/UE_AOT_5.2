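; Player controller for the grappling hook game that creates and manages the in-game UI widget.
; On BeginPlay the local controller creates UI_IngameWidget and adds it to the viewport.
; The ShowMenu input action forwards press and release to the widget's show and hide menu handlers.
; A T key press removes the widget from its parent.
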(event EventBeginPlay
  (bind _self self)
  (if (Pawn|IsLocalController _self)
    (bind _returnvalue (UserInterface|CreateWidget "/Game/GrapplingHook/Blueprints/UI/UI_IngameWidget.UI_IngameWidget_C" _self))
    (bind _output_get (Variables|Default|SetUI _returnvalue))
    (UserInterface|Viewport|AddtoViewport _output_get 0)))

(event Input|ActionEvents|InputActionShowMenu
  (params (Key :type Key%20Structure :default "None"))
  (bind _ui (Variables|Default|GetUI))
  (bind _ui_2 (Variables|Default|GetUI))
  (:Pressed
    (Utilities|IsValid _ui_2
      (:Is%20Valid
        (Default|OnShowMenu _ui_2))))
  (:Released
    (Utilities|IsValid _ui
      (:Is%20Valid
        (Default|OnHideMenu _ui)))))

(event Input|KeyboardEvents|T
  (params (Key :type Key%20Structure :default "None"))
  (:Pressed
    (Widget|RemovefromParent (Variables|Default|GetUI))))

(fn ConstructionScript)
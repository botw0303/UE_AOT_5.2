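; Example playable character for the grappling hook system, a child Blueprint that inherits its functionality from BP_GrapplingHookCharacter.
; BeginPlay and Tick only call the parent implementations.
; The construction script runs the parent's, then attaches the left and right gear components to the LegLeft and LegRight mesh sockets, snapping rotation while keeping relative location and scale.
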(event EventBeginPlay
  ;[0.3265 1 0.4314] See BP_GrapplingHookCharacter for functionality
  (|CallParentFunction))

(event EventTick
  (params (DeltaSeconds :type Float%20%28single-precision%29))
  ;[0.3265 1 0.4314] See BP_GrapplingHookCharacter for functionality
  (|CallParentFunction DeltaSeconds))

(fn ConstructionScript
  (|CallParentFunction)
  ;[1 0.4643 0.7015] Attach the character gear to the specified sockets ("LegLeft" and "LegRight")
  (Transformation|AttachComponentToComponent (Variables|Default|GetGearLeft) (Variables|Character|GetMesh) "LegLeft" "KeepRelative" "SnapToTarget" "KeepRelative" true)
  (Transformation|AttachComponentToComponent (Variables|Default|GetGearRight) (Variables|Character|GetMesh) "LegRight" "KeepRelative" "SnapToTarget" "KeepRelative" true))